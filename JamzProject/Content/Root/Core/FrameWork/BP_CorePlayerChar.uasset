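; BP_CorePlayerChar is a player character Blueprint that holds health and has key-driven hooks into the two-player health GUI.
; The construction script sets Health to MaxHealth, and BeginPlay caches MainGUI from CoreGameMode.
; The U and I keys call SetHealthPercentage on MainGUI for the Player 2 and Player 1 GUI elements respectively, without changing Health.
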(event `self.ReceiveBeginPlay`
  (bind _ascore_game_mode (cast `/Game/Root/Core/FrameWork/CoreGameMode` (`GameplayStatics.GetGameMode`)))
  (set `self.MainGUI` (`/Game/Root/Core/FrameWork/CoreGameMode.mainGUI` _ascore_game_mode)))

(event `Key|U`
  (params (Key :type "Key Structure"))
  (bind _maingui (`self.MainGUI`))
  (:`Pressed`
    (`/Game/Root/Assets/Blueprints/Main.SetHealthPercentage` _maingui (`/Game/Root/Assets/Blueprints/Main.GUI_Player2` _maingui))))

(event `Key|I`
  (params (Key :type "Key Structure"))
  (bind _maingui (`self.MainGUI`))
  (:`Pressed`
    (`/Game/Root/Assets/Blueprints/Main.SetHealthPercentage` _maingui (`/Game/Root/Assets/Blueprints/Main.GUI_Player1` _maingui))))

(fn `UserConstructionScript`
  (set `self.health` (`self.maxHealth`)))