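; BP_PoolKidBase is a pool kid AI character that runs the BT_Kid behavior tree on BeginPlay and switches between swimming and walking.
; Swimming loops a timeline that moves the mesh vertically while the swim flag is set.
; OnWalking clears the flag, briefly simulates capsule physics with an upward impulse, and plays a mesh-offset timeline whose lerp alpha is fixed at zero, leaving the mesh in place.
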(event `self.ReceiveBeginPlay`
  (`AIController.RunBehaviorTree` (`AIBlueprintHelperLibrary.GetAIController` self) "/Game/Root/Core/Ai/BT_Kid.BT_Kid"))

(event `Swimming`
  (set `self.Swimmig` true)
  (bind (_direction _floattrack) (`Timeline|Timeline_0` :!label _label)
    (:`Update`
      (`SceneComponent.K2_SetRelativeLocation` (`self.Mesh`) (`KismetMathLibrary.VLerp` (0.0 0.0 -60.0) (0.0 0.0 -40.0) _floattrack) false false))
    (:`Finished`
      (if (`self.Swimmig`)
        (goto _label :!via `PlayFromStart`)))))

(event `OnWalking`
  (bind _capsulecomponent (`self.CapsuleComponent`))
  (set `self.Swimmig` false)
  (`|ExecutionSequence`
    (:`then_0`
      (`Timeline|Timeline_1` :!via `PlayFromStart`
        (:`Update`
          (`SceneComponent.K2_SetRelativeLocation` (`self.Mesh`) (`KismetMathLibrary.VLerp` (`SceneComponent.RelativeLocation` (`self.Mesh`)) (0.0 0.0 -80.0)) false false))))
    (:`then_1`
      (`PrimitiveComponent.SetSimulatePhysics` _capsulecomponent true)
      (`PrimitiveComponent.AddImpulseAtLocation` _capsulecomponent (0.0 0.0 65000.0) (`SceneComponent.RelativeLocation` _capsulecomponent) "Character1_Hips")
      (`KismetSystemLibrary.PrintString` "FLYYG")
      (`KismetSystemLibrary.Delay` 0.5)
      (`PrimitiveComponent.SetSimulatePhysics` (`self.CapsuleComponent`) false))))

(fn `UserConstructionScript`)