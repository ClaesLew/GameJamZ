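; Beach ball actor (Badboll) that briefly turns physical when the player character enters its trigger sphere.
; A timeline drives the ball's relative height in a small vertical bob, and the overlap stops it.
; The overlap also enables physics simulation and collision on the ball, then switches both off again after a one-second delay.
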(event `self.ReceiveBeginPlay`)

(event `self.ReceiveActorBeginOverlap`
  (params (OtherActor :type "Actor Object Reference")))

(event `self.Sphere.OnComponentBeginOverlap`
  (params (OverlappedComponent :type "PrimitiveComponent Object Reference") (OtherActor :type "Actor Object Reference") (OtherComp :type "PrimitiveComponent Object Reference") (OtherBodyIndex :type Integer) (bFromSweep :type Boolean) (SweepResult :type "HitResult Structure (by ref)"))
  (bind _badboll (`self.Badboll`))
  (cast `/Game/Root/Core/FrameWork/BP_CorePlayerChar` OtherActor)
  (`|ExecutionSequence`
    (:`then_0`
      (bind (_direction _float) (`Timeline|Timeline_0` :`NewTime` 0.0 :!via `Stop`)
        (:`Update`
          (`SceneComponent.K2_SetRelativeLocation` (`self.Badboll`) (`KismetMathLibrary.VLerp` (0.0 0.0 10.0) (0.0 0.0 -10.0) _float) false false))))
    (:`then_1`
      (`PrimitiveComponent.SetSimulatePhysics` _badboll true)
      (`PrimitiveComponent.SetCollisionEnabled` _badboll "QueryAndPhysics")
      (`KismetSystemLibrary.Delay` 1.0)
      (`PrimitiveComponent.SetSimulatePhysics` _badboll false)
      (`PrimitiveComponent.SetCollisionEnabled` (`self.Badboll`) "NoCollision"))))

(fn `UserConstructionScript`)